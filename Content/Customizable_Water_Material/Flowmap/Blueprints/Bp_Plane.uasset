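; Paintable plane actor that records positions and velocities into a flowmap render target for the customizable water material.
; The construction script creates a dynamic brush material instance, and BeginPlay clears the render target to black.
; The Draw event converts a world position into plane UV space using the mesh bounds, passes it with velocity and radius to the brush, then renders that material into the flowmap.
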(event `Draw`
  (params (Position :type "Vector Structure") (Valocity :type "Vector Structure") (`Brush size` :type "Float (double-precision)"))
  (bind _brush (`self.Brush`))
  (bind _returnvalue_x (`KismetMathLibrary.BreakVector` (`SceneComponent.K2_GetComponentScale` (`self.Plane`))))
  (`MaterialInstanceDynamic.SetVectorParameterValue` (`self.Brush`) "Position" (`KismetMathLibrary.Conv_VectorToLinearColor` (+ (/ (`KismetMathLibrary.InverseTransformLocation` (`self.GetTransform`) Position) (/ (* (.x (`.BoxExtent` (`KismetSystemLibrary.GetComponentBounds` (`self.Plane`)))) 2.0) _returnvalue_x)) 0.5)))
  (`MaterialInstanceDynamic.SetVectorParameterValue` _brush "Velocity" (`KismetMathLibrary.Conv_VectorToLinearColor` Valocity))
  (`MaterialInstanceDynamic.SetScalarParameterValue` _brush "Radius" `Brush size`)
  (`KismetRenderingLibrary.DrawMaterialToRenderTarget` "/Game/Customizable_Water_Material/Flowmap/RT_FlowMap.RT_FlowMap" (`self.Brush`)))

(event `self.ReceiveBeginPlay`
  (`KismetRenderingLibrary.ClearRenderTarget2D` "/Game/Customizable_Water_Material/Flowmap/RT_FlowMap.RT_FlowMap"))

(fn `UserConstructionScript`
  (bind _returnvalue (`KismetMaterialLibrary.CreateDynamicMaterialInstance` "/Game/Customizable_Water_Material/Flowmap/M_Brush.M_Brush"))
  (set `self.Brush` _returnvalue))