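; BP_PaintPawn is a mouse-driven pawn for painting onto a Bp_Plane actor, part of a water material flowmap tool.
; Each tick it traces under the cursor, derives mouse velocity from the change in hit location, and moves a sphere marker to that point.
; While the left button is held, it passes position, intensity-scaled velocity and brush size to the plane's Draw; right-button state is tracked but unused.
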(event `self.ReceiveBeginPlay`
  (set `PlayerController.bShowMouseCursor` true (`GameplayStatics.GetPlayerController` 0))
  (bind _outactors (`GameplayStatics.GetAllActorsOfClass` "/Game/Customizable_Water_Material/Flowmap/Blueprints/Bp_Plane.Bp_Plane_C"))
  (set `self.Plane` (`|GetArrayItem` _outactors)))

(event `Key|LeftMouseButton`
  (params (Key :type "Key Structure"))
  (:`Pressed`
    (set `self.LeftmouseDown` true))
  (:`Released`
    (set `self.LeftmouseDown` false)))

(event `Key|RightMouseButton`
  (params (Key :type "Key Structure"))
  (:`Pressed`
    (set `self.RightmouseDown` true))
  (:`Released`
    (set `self.RightmouseDown` false)))

(event `self.ReceiveTick`
  (params (DeltaSeconds :type "Float (single-precision)"))
  (`self.Trace Under Mouse`)
  (`self.Update sphere loc`)
  (if (`self.LeftmouseDown`)
    (bind _output_get (set `self.Velocity` (* (`self.Mouse Velocity`) (`self.Intensity`))))
    (`/Game/Customizable_Water_Material/Flowmap/Blueprints/Bp_Plane.Draw` (`self.Plane`) (`self.Position`) _output_get (`self.Brush Size`))))

(fn `Trace Under Mouse`
  (bind (_hitresult _returnvalue) (`PlayerController.GetHitResultUnderCursorByChannel` (`GameplayStatics.GetPlayerController` 0) "TraceTypeQuery1" true))
  (if _returnvalue
    (set `self.Mouse Velocity` (- (`.Location` (`GameplayStatics.BreakHitResult` _hitresult)) (`self.Position`)))
    (set `self.Position` (`.Location` (`GameplayStatics.BreakHitResult` _hitresult)))
    (return)))

(fn `Update sphere loc`
  (`SceneComponent.K2_SetWorldLocationAndRotation` :`self` (`self.Sphere`) :`NewLocation` (`self.Position`)))

(fn `UserConstructionScript`)